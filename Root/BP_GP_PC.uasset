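; BP_GP_PC is a player controller Blueprint that toggles the game's pause menu with the P key.
; Pausing shows the cursor, creates a new WBP_pause widget, switches input to Game and UI focused on it, and plays its start animation.
; Unpausing hides the cursor, restores game-only input, and calls the widget's reverse animation immediately before removing it from the viewport, without waiting for it to finish.
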(event Input|KeyboardEvents|P
  (params (Key :type Key%20Structure :default "None"))
  (bind _returnvalue (Game|GetPlayerController 0))
  (:Pressed
    (if (Game|IsGamePaused)
      (Game|SetGamePaused false)
      (Variables|Default|SetbShowMouseCursor false)
      (Default|PauseAnimReverce (stale _returnvalue_2))
      (Widget|RemovefromParent (stale _returnvalue_2))
      (Input|SetInputModeGameOnly _returnvalue)
      (else
        (Game|SetGamePaused true)
        (Variables|Default|SetbShowMouseCursor true)
        (bind _returnvalue_2 (UserInterface|CreateWidget "/Game/Root/PauseUI/WBP_pause.WBP_pause_C"))
        (UserInterface|Viewport|AddtoViewport _returnvalue_2 0)
        (Input|SetInputModeGameandUI _returnvalue _returnvalue_2 "DoNotLock" true)
        (Default|PauseAnimStart _returnvalue_2)))))

(fn ConstructionScript)