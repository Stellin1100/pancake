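; BP_Enemy2 is an AI enemy pawn that wanders at random until it spots the player, then chases them.
; Tick issues either a random-point move or a faster AIMoveTo toward the player, based on a See flag.
; PawnSensing sets See on seeing a player-controlled pawn, and nothing here clears it.
; A DeathAnim event plays a dying montage when AI_HP in the My_GI game instance is depleted.
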(event OnSeePawn(PawnSensing)
  (params (Pawn :type Pawn%20Object%20Reference))
  ;[0.01938 0.01938 0.01938] Check if it is our character and set "see?" variable true
  (if (Pawn|IsPlayerControlled Pawn)
    (Variables|Default|SetSee? true)
    (Utilities|FlowControl|DoOnce false)))

(event Custom|Enemy2_Random%20Walk
  ;[0.01938 0.01938 0.01938] Walk Rendom
  (AI|AIMoveTo self (.RandomLocation (AI|Navigation|GetRandomReachablePointinRadius (Transformation|GetActorLocation) 4e+03 0 0)) 0 5.0 false))

(event Custom|RunIntoPlayer
  ;[0.01938 0.01938 0.01938] Run into Player
  (Variables|/Script/Engine.CharacterMovementComponent|SetMaxWalkSpeed (Variables|Character|GetCharacterMovement) 6e+02)
  (AI|AIMoveTo self "0, 0, 0" (Game|GetPlayerCharacter 0) 5.0 false))

(event Custom|DeathAnim
  ;[0.01938 0.01938 0.01938] AI_Death animation
  (bind _asmy_gi (Utilities|Casting|CastToMy_GI (Game|GetGameInstance)))
  (if (<= (.ai_hp (Variables|/Game/Root/Game_Instance/My_GI.My_GI_C|GetMyST _asmy_gi)) 0)
    (Animation|PlayAnimMontage self "/Game/Root/AI_Enemies/AI_Enemy2/Anims/Animations/Dying_Backwards_Montage.Dying_Backwards_Montage" 1.0 "None")))

(event EventTick
  (params (DeltaSeconds :type Float%20%28single-precision%29))
  (if (Variables|Default|GetSee?)
    (CallFunction|RunIntoPlayer)
    (else
      (CallFunction|Enemy2RandomWalk))))

(fn ConstructionScript)