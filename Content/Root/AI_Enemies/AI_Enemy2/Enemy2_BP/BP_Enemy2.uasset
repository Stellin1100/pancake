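; BP_Enemy2 is an AI enemy character that wanders, chases the player and dies when health runs out.
; Tick runs random reachable-point moves until PawnSensing sees the player, then switches permanently to chasing.
; Reaching the player applies damage and calls CallED1 and DeathAction on BP_MyGI.
; Taking damage plays a hit montage, whose returned length becomes walk speed; death enables mesh physics and destroys the actor after a delay.
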(event OnSeePawn(PawnSensing)
  (params (Pawn :type Pawn%20Object%20Reference))
  ;[0.01938 0.01938 0.01938] Check if it is our character and set "see?" variable true
  (if (Pawn|IsPlayerControlled Pawn)
    (Variables|Default|SetSee? true)
    (Utilities|FlowControl|DoOnce false)))

(event Custom|Enemy2_Random%20Walk
  ;[0.01938 0.01938 0.01938] Walk Rendom
  (AI|AIMoveTo self (.RandomLocation (AI|Navigation|GetRandomReachablePointinRadius (Transformation|GetActorLocation) 4e+03 0 0)) 0 5.0 false))

(event Custom|RunIntoPlayer
  (bind _returnvalue (Game|GetPlayerCharacter 0))
  ;[0.01938 0.01938 0.01938] Run into Player
  (Variables|/Script/Engine.CharacterMovementComponent|SetMaxWalkSpeed (Variables|Character|GetCharacterMovement) 3e+02)
  (AI|AIMoveTo self "0, 0, 0" _returnvalue 5.0 false
    (:OnSuccess
      (Game|Damage|ApplyDamage _returnvalue 15.0 0 self)
      (bind _asbp_my_gi (Utilities|Casting|CastToBP_MyGI (Game|GetGameInstance)))
      (Default|CallED1 _asbp_my_gi)
      (Default|DeathAction _asbp_my_gi))))

(event Custom|AI_Death
  ;[0.01938 0.01938 0.01938] AI Death
  (Components|Animation|PlayAnimation (Variables|Character|GetMesh) "/Game/Root/AI_Enemies/AI_Enemy2/Anims/Animations/Dying_Backwards.Dying_Backwards" true)
  (Physics|SetSimulatePhysics (Variables|Character|GetMesh) true)
  (Pawn|Components|CharacterMovement|DisableMovement (Variables|Character|GetCharacterMovement))
  (Utilities|FlowControl|Delay 5.0)
  (Actor|DestroyActor))

(event EventTick
  (params (DeltaSeconds :type Float%20%28single-precision%29))
  (if (Variables|Default|GetSee?)
    (CallFunction|RunIntoPlayer)
    (else
      (CallFunction|Enemy2RandomWalk))))

(event Game|Damage|EventAnyDamage
  (params (Damage :type Float%20%28single-precision%29) (DamageType :type Damage%20Type%20Object%20Reference) (InstigatedBy :type Controller%20Object%20Reference) (DamageCauser :type Actor%20Object%20Reference))
  ;[0.01938 0.01938 0.01938] AI Get Hit
  (bind _output_get (Variables|Default|Sethp (- (Variables|Default|Gethp) Damage)))
  (Development|PrintString (Utilities|String|ToString(Float) _output_get))
  (bind _returnvalue (Animation|PlayAnimMontage "/Game/Root/AI_Enemies/AI_Enemy2/Anims/Animations/Hit_To_Body_Montage.Hit_To_Body_Montage" 1.0 "None"))
  (Variables|/Script/Engine.CharacterMovementComponent|SetMaxWalkSpeed (Variables|Character|GetCharacterMovement) _returnvalue)
  (if (<= (Variables|Default|GetHP) 0.0)
    (CallFunction|AIDeath)))

(fn ConstructionScript)