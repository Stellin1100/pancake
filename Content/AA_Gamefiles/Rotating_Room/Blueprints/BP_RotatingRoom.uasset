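; BP_RotatingRoom is an actor that rearranges room components when its trigger box is overlapped.
; On overlap it checks that player character 0, rather than the overlapping actor, implements BP_Interface.
; It then instantly snaps Room2 through Room5 to hardcoded relative locations and rotations, with no interpolation or reset.
; An unconnected node that would set Room1's mesh from a Rooms array never runs.
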(event OnComponentBeginOverlap(Box)
  (params (OverlappedComponent :type Primitive%20Component%20Object%20Reference) (OtherActor :type Actor%20Object%20Reference) (OtherComp :type Primitive%20Component%20Object%20Reference) (OtherBodyIndex :type Integer) (bFromSweep :type Boolean) (SweepResult :type Hit%20Result%20Structure%20%28by%20ref%29))
  (if (Utilities|DoesObjectImplementInterface (Game|GetPlayerCharacter 0) "/Game/Rotating_Room/Blueprints/BP_Interface.BP_Interface_C")
    (Utilities|FlowControl|Sequence
      (:then_0
        (Transformation|SetRelativeLocationAndRotation (Variables|Default|GetRoom_2) "230.000000,-530.000000,120.000000" "180.000000,180.000000, 0" false false))
      (:then_1
        (Transformation|SetRelativeLocationAndRotation (Variables|Default|GetRoom_3) "840.000000,560.000000,30.000000" "0,180.000000, 0" false false))
      (:then_2
        (Transformation|SetRelativeLocationAndRotation (Variables|Default|GetRoom_4) "1060.000000,320.000000,30.000000" "0, 0,180.000000" false false))
      (:then_3
        (Transformation|SetRelativeLocationAndRotation (Variables|Default|GetRoom_5) "580.000000,-225.000000,30.000000" "0, 0, 0" false false)))))

(fn ConstructionScript)